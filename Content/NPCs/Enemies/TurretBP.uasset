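; Enemy turret pawn that chases the RuneHunter player character on sight and shoots projectiles at them.
; When PawnSensing spots the player, it snaps its rotation to face them and uses AIMoveTo to close to within an acceptance radius.
; On a successful move, it spawns a TurretProjectileBP at the spawn point and launches it forward with an impulse.
; A boolean flag and short delay throttle the fire rate.
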(event `self.PawnSensing.OnSeePawn`
  (params (Pawn :type "Pawn Object Reference"))
  (bind _asrune_hunter_character_bp (cast `/Game/Character/RuneHunterCharacterBP` Pawn))
  (`self.K2_SetActorRotation` (`KismetMathLibrary.FindLookAtRotation` (`self.K2_GetActorLocation`) (`self.K2_GetActorLocation` _asrune_hunter_character_bp)))
  (`|AIMoveTo` self (0.0 0.0 0.0) _asrune_hunter_character_bp 500.0
    (:`OnSuccess`
      (if (`self.SpawnProjectile`)
        (bind _returnvalue (`|SpawnActorFromClass` "/Game/NPCs/Enemies/TurretProjectileBP.TurretProjectileBP_C" (`SceneComponent.K2_GetComponentToWorld` (`self.ProjectileSpawnLocation`)) "Undefined" "OverrideRootScale" null null))
        (`PrimitiveComponent.AddImpulse` (`/Game/NPCs/Enemies/TurretProjectileBP.Sphere` _returnvalue) (* (`SceneComponent.GetForwardVector` (`self.CapsuleComponent`)) (`self.ShootSpeed`)) "None" true)
        (set `self.SpawnProjectile` false)
        (`KismetSystemLibrary.Delay` 0.2)
        (set `self.SpawnProjectile` true)))))

(fn `UserConstructionScript`)