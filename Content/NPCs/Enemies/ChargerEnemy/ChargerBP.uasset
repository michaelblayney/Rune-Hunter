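; ChargerBP is an enemy that deals contact damage to the player and can be killed.
; Sphere overlaps with RuneHunterCharacterBP toggle a Colliding flag.
; While it is set, Tick prints a debug "Hit" and calls DamagePlayer on the game instance, so damage lands every frame rather than per second.
; TakeDamage subtracts from Health and destroys the actor at zero or below; no charging movement is defined here.
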(event `self.Sphere.OnComponentBeginOverlap`
  (params (OverlappedComponent :type "PrimitiveComponent Object Reference") (OtherActor :type "Actor Object Reference") (OtherComp :type "PrimitiveComponent Object Reference") (OtherBodyIndex :type Integer) (bFromSweep :type Boolean) (SweepResult :type "HitResult Structure (by ref)"))
  (cast `/Game/Character/RuneHunterCharacterBP` OtherActor)
  (set `self.Colliding` true))

(event `self.Sphere.OnComponentEndOverlap`
  (params (OverlappedComponent :type "PrimitiveComponent Object Reference") (OtherActor :type "Actor Object Reference") (OtherComp :type "PrimitiveComponent Object Reference") (OtherBodyIndex :type Integer))
  (cast `/Game/Character/RuneHunterCharacterBP` OtherActor)
  (set `self.Colliding` false))

(event `self.ReceiveTick`
  (params (DeltaSeconds :type "Float (single-precision)"))
  (if (`self.Colliding`)
    (`KismetSystemLibrary.PrintString` "Hit")
    (bind _asrune_hunter_game_instance_bp (cast `/Game/Blueprints/RuneHunterGameInstanceBP` (`GameplayStatics.GetGameInstance`)))
    (`/Game/Blueprints/RuneHunterGameInstanceBP.DamagePlayer` _asrune_hunter_game_instance_bp (`self.Damage`))))

(fn `TakeDamage`
  (params (Damage :type Integer))
  (locals (Temp :type Integer))
  (bind _output_get (set `local.Temp` (- (`self.Health`) Damage)))
  (if (<= _output_get 0)
    (`self.K2_DestroyActor`)
    (else
      (set `self.Health` (`local.Temp`)))))

(fn `UserConstructionScript`)