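; Projectile actor fired by the turret enemy, made up of Fireball and Sphere components.
; On BeginPlay it starts a two-second delay, then destroys itself.
; Each Tick shrinks both components by one percent of their current scale, so the shot visibly burns out as it travels, at a rate tied to frame rate.
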(event `self.ReceiveBeginPlay`
  ;[1 1 1] Projectile burns out over 2 seconds from creation
  (`KismetSystemLibrary.Delay` 2.0)
  (`self.K2_DestroyActor`))

(event `self.ReceiveTick`
  (params (DeltaSeconds :type "Float (single-precision)"))
  (bind _sphere (`self.Sphere`))
  (bind _fireball (`self.Fireball`))
  ;[1 1 1] Shrink projectile as it travels
  (`|ExecutionSequence`
    (:`then_0`
      (`SceneComponent.SetWorldScale3D` _fireball (* (`SceneComponent.K2_GetComponentScale` _fireball) 0.99)))
    (:`then_1`
      (`SceneComponent.SetWorldScale3D` _sphere (* (`SceneComponent.K2_GetComponentScale` _sphere) 0.99)))))

(fn `UserConstructionScript`)