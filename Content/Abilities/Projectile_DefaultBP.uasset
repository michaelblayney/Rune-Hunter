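; Default player projectile Blueprint that damages what it hits and removes itself once off-screen.
; Tick projects its location to screen space and destroys it outside the viewport bounds.
; Collision overlaps ignore the player character and bat, boss and dragon projectiles through exact class checks.
; Any other overlap destroys the projectile and passes the hit actor to DamageEnemy on RuneHunterGameInstanceBP, which handles the damage.
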(event `self.ReceiveTick`
  (params (DeltaSeconds :type "Float (single-precision)"))
  (bind (_x _y) (`KismetMathLibrary.BreakVector2D` (`WidgetLayoutLibrary.GetViewportSize`)))
  (bind (_x_2 _y_2) (`KismetMathLibrary.BreakVector2D` (`PlayerController.ProjectWorldLocationToScreen` (`GameplayStatics.GetPlayerController` 0) (`self.K2_GetActorLocation`) false)))
  (if (or (< _x_2 0.0) (< _y_2 0.0) (> _x_2 _x) (> _y_2 _y))
    (`self.K2_DestroyActor`)))

(event `self.ProjCollisionComponent.OnComponentBeginOverlap`
  (params (OverlappedComponent :type "PrimitiveComponent Object Reference") (OtherActor :type "Actor Object Reference") (OtherComp :type "PrimitiveComponent Object Reference") (OtherBodyIndex :type Integer) (bFromSweep :type Boolean) (SweepResult :type "HitResult Structure (by ref)"))
  (bind _returnvalue (`GameplayStatics.GetObjectClass` OtherActor))
  ;[1 1 1] Prevent the projectile colliding with player when fired
  (if (not (== _returnvalue "/Game/Character/RuneHunterCharacterBP.RuneHunterCharacterBP_C"))
    ;[1 1 1] Prevents player projectiles colliding with enemy projectiles
    (if (== _returnvalue "/Game/NPCs/Enemies/Bat/BatProjectile.BatProjectile_C")
      _
      (elif (== _returnvalue "/Game/NPCs/Enemies/Boss/BossProjectile.BossProjectile_C")
        _
        (elif (not (== _returnvalue "/Game/NPCs/Enemies/ChargerEnemy/DragonVomit.DragonVomit_C"))
          (`self.K2_DestroyActor`)
          (bind _asrune_hunter_game_instance_bp (cast `/Game/Blueprints/RuneHunterGameInstanceBP` (`GameplayStatics.GetGameInstance`)))
          (`/Game/Blueprints/RuneHunterGameInstanceBP.DamageEnemy` _asrune_hunter_game_instance_bp OtherActor))))))

(fn `UserConstructionScript`)