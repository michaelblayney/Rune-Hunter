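; Trail actor that draws a spline-mesh trail with collision behind the player while the rune hunter ability is active.
; A left-press event opens a Tick gate if CanShoot, adding spline points at the player's feet and appending spline mesh segments, which are cleared once the trail exceeds TrailLength.
; TrailCollision actors spawn only on every Nth point for performance, with the oldest culled.
; TrailStopandDestroy shrinks the trail until the actor destroys itself.
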(event `self.ReceiveTick`
  (params (DeltaSeconds :type "Float (single-precision)"))
  (bind _spline (`self.Spline`))
  (bind _splinemeshes (`self.SplineMeshes`))
  (bind _spline_2 (`self.Spline`))
  ;[1 1 1] Continuous loop as long as trail exists
  (`self.Remove End of Collision Trail`)
  (`/Engine/EditorBlueprintResources/StandardMacros.Gate` true :!label _label
    (:`Exit`
      ;[1 1 1] Drawing spline
      (if (and (== (`SplineComponent.GetNumberOfSplinePoints` (`self.Spline`)) 2) (`self.DestroyNow`))
        ;[1 1 1] Destroy collision and trail when the trail is at minimum length
        (for _array_element (`self.CollisionTrail`)
          (`self.K2_DestroyActor` _array_element))
        (`self.K2_DestroyActor`)
        (else
          (if (or (stale `Trail Stop and Destroy` _output_get) (> (`SplineComponent.GetNumberOfSplinePoints` (`self.Spline`)) (`self.TrailLength`)))
            ;;[1 1 1] Remove end of trail overtime
            ;;;[1 1 1] Remove end of spline
            (for _index (range 2)
              (`SplineComponent.RemoveSplinePoint` (`self.Spline`) _index true))
            ;;;[1 1 1] Clear Spline Mesh so new one can be drawn
            (for _array_element_2 _splinemeshes
              (`ActorComponent.K2_DestroyComponent` _array_element_2))
            (`KismetArrayLibrary.Array_Clear` _splinemeshes))
          (`SplineComponent.AddSplinePoint` _spline (`KismetMathLibrary.TransformLocation` (`KismetMathLibrary.MakeTransform` (0.0 0.0 -100.0)) (`self.K2_GetActorLocation` (`GameplayStatics.GetPlayerPawn` 0))) "Local" true) ; Is the spline itself, this part is not being rendered in runtime
          (for _index_2 (range (+ (- (`SplineComponent.GetNumberOfSplinePoints` _spline) 2) 1))
            ;;[1 1 1] Spline Mesh is what is being displayed
            (bind _returnvalue (`AddComponent|NODE_AddSplineMeshComponent-1` :`bManualAttachment` true)) ; Set to manual attachment to stop trail growing over time
            (`KismetArrayLibrary.Array_Add` (`self.SplineMeshes`) _returnvalue)
            (`self.Create Collision Trail` _index_2)
            (`SplineMeshComponent.SetForwardAxis` _returnvalue "X" true)
            (bind (_location _tangent) (`SplineComponent.GetLocationAndTangentAtSplinePoint` _spline_2 _index_2 "Local"))
            (bind (_location_2 _tangent_2) (`SplineComponent.GetLocationAndTangentAtSplinePoint` _spline_2 (+ _index_2 1) "Local"))
            (`SplineMeshComponent.SetStartAndEnd` _returnvalue _location _tangent _location_2 _tangent_2 true)))))))

(event `Left Mouse Pressed`
  ;[1 1 1] When mouse to pressed, then trail actor is spawned and should start drawing trail
  (bind _asrune_hunter_character_bp (cast `/Game/Character/RuneHunterCharacterBP` (`GameplayStatics.GetPlayerPawn` 0)))
  (if (`/Game/Character/RuneHunterCharacterBP.CanShoot` _asrune_hunter_character_bp)
    (`SplineComponent.ClearSplinePoints` (`self.Spline`) true)
    (goto _label :!via `Open`)
    (else
      (goto _label :!via `Close`))))

(event `Trail Stop and Destroy`
  ;[1 1 1] Drawing spline
  ;;[1 1 1] Is called when mouse button has been released
  (bind _output_get (set `self.DestroyNow` true)))

(fn `Create Collision Trail`
  (params (Index :type Integer))
  (bind _spline (`self.Spline`))
  ;[1 1 1] Only draws a collision box on every Nth point, lowering performance cost
  (if (== (mod Index (`self.CollisionPerformanceModifier`)) 0)
    (bind _returnvalue (`|SpawnActorFromClass` "/Game/Abilities/trailCollision.trailCollision_C" (`KismetMathLibrary.MakeTransform` (`SplineComponent.GetLocationAtSplinePoint` _spline Index "Local") (`SplineComponent.GetRotationAtSplinePoint` _spline Index "Local")) "AlwaysSpawn" "OverrideRootScale" null null))
    (`KismetArrayLibrary.Array_Add` (`self.CollisionTrail`) _returnvalue)))

(fn `Remove End of Collision Trail`
  (bind _collisiontrail (`self.CollisionTrail`))
  (while (> (`KismetArrayLibrary.Array_Length` _collisiontrail) (/ (`self.TrailLength`) (`self.CollisionPerformanceModifier`)))
    (`self.K2_DestroyActor` (`|GetArrayItem` _collisiontrail))
    (`KismetArrayLibrary.Array_Remove` _collisiontrail)))

(fn `UserConstructionScript`)