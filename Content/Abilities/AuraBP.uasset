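; AuraBP is an ability aura actor that follows the player pawn and fades out over its life span.
; BeginPlay creates a dynamic material instance for the aura mesh.
; After the life span is set, JustAfterSpawning stretches the FadeOut timeline to match it and drives the material's Opacity.
; Tick snaps the actor to player pawn 0; the collision hit event is an empty stub.
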(event `self.ReceiveBeginPlay`
  ;[1 1 1] Create dynamic material to fade out during aura's life span
  (bind _returnvalue (`KismetMaterialLibrary.CreateDynamicMaterialInstance` (`PrimitiveComponent.GetMaterial` (`self.AuraMeshComponent`) 0)))
  (bind _output_get (set `self.FadeMat` _returnvalue))
  (`PrimitiveComponent.SetMaterial` (`self.AuraMeshComponent`) 0 _output_get))

(event `JustAfterSpawning`
  ;[1 1 1] Is called after setting life span of aura
  (`TimelineComponent.SetTimelineLength` (`self.FadeOut`) (`self.GetLifeSpan`))
  (bind (_direction _alpha) (`Timeline|FadeOut`) ; Fade out used for material, could be used for damage as well
    (:`Update`
      (`MaterialInstanceDynamic.SetScalarParameterValue` (`self.FadeMat`) "Opacity" _alpha))))

(event `self.ReceiveTick`
  (params (DeltaSeconds :type "Float (single-precision)"))
  ;[1 1 1] Translating aura to character's position
  (`self.K2_SetActorLocation` (`self.K2_GetActorLocation` (`GameplayStatics.GetPlayerPawn` 0))))

(event `self.AuraCollisionComponent.OnComponentHit`
  (params (HitComponent :type "PrimitiveComponent Object Reference") (OtherActor :type "Actor Object Reference") (OtherComp :type "PrimitiveComponent Object Reference") (NormalImpulse :type "Vector Structure") (Hit :type "HitResult Structure (by ref)")))

(fn `UserConstructionScript`)