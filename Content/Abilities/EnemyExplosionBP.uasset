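; EnemyExplosionBP is an explosion aura ability that damages enemies it touches and fades out over its lifetime.
; BeginPlay gives the aura mesh a dynamic material, and JustAfterSpawning, meant to follow setting the life span, stretches the FadeOut timeline to that span to drive opacity.
; Collision overlaps pass the other actor to RuneHunterGameInstanceBP's DamageEnemy, independent of the fade.
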(event `self.ReceiveBeginPlay`
  ;[1 1 1] Create dynamic material to fade out during aura's life span
  (bind _returnvalue (`KismetMaterialLibrary.CreateDynamicMaterialInstance` (`PrimitiveComponent.GetMaterial` (`self.AuraMeshComponent`) 0)))
  (bind _output_get (set `self.FadeMat` _returnvalue))
  (`PrimitiveComponent.SetMaterial` (`self.AuraMeshComponent`) 0 _output_get))

(event `JustAfterSpawning`
  ;[1 1 1] Is called after setting life span of aura
  (`TimelineComponent.SetTimelineLength` (`self.FadeOut`) (`self.GetLifeSpan`))
  (bind (_direction _alpha) (`Timeline|FadeOut`) ; Fade out used for material, could be used for damage as well
    (:`Update`
      (`MaterialInstanceDynamic.SetScalarParameterValue` (`self.FadeMat`) "Opacity" _alpha))))

(event `self.AuraCollisionComponent.OnComponentBeginOverlap`
  (params (OverlappedComponent :type "PrimitiveComponent Object Reference") (OtherActor :type "Actor Object Reference") (OtherComp :type "PrimitiveComponent Object Reference") (OtherBodyIndex :type Integer) (bFromSweep :type Boolean) (SweepResult :type "HitResult Structure (by ref)"))
  ;[1 1 1] Damage enemies that are hit by the aura
  (bind _asrune_hunter_game_instance_bp (cast `/Game/Blueprints/RuneHunterGameInstanceBP` (`GameplayStatics.GetGameInstance`)))
  (`/Game/Blueprints/RuneHunterGameInstanceBP.DamageEnemy` _asrune_hunter_game_instance_bp OtherActor))

(fn `UserConstructionScript`)