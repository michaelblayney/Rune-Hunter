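; Game instance for Rune Hunter that builds a randomized branching dungeon layout on Init and tracks the player's layer across levels.
; It randomly picks two unique first-layer rooms and four unique second-layer rooms, excluding each parent from its children's pool.
; GetNextRooms returns two destinations from the current layer and level name, using fixed tiles for later layers.
; IncrimentLayer advances the layer, wrapping to zero after the last.
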(event `self.ReceiveInit`
  (`self.Determine Room Layout`))

(fn `Determine Room Layout`
  (locals (TempRoomPool :type "Array of Name"))
  ;[1 1 1] Build first layer of the dungeon
  (while (< (`KismetArrayLibrary.Array_Length` (`self.Layer1`)) 2)
    (`KismetArrayLibrary.Array_AddUnique` (`self.Layer1`) (`KismetArrayLibrary.Array_Random` (`self.RoomNames`))))
  ;[1 1 1] Build second layer of the dungeon
  (while (< (`KismetArrayLibrary.Array_Length` (`self.Layer2`)) 4)
    ;;[1 1 1] Prevent players walking into a room they just came out of
    (if (< (`KismetArrayLibrary.Array_Length` (`self.Layer2`)) 2)
      (bind _output_get (set `local.TempRoomPool` (`self.RoomNames`)))
      (`KismetArrayLibrary.Array_RemoveItem` _output_get (`|GetArrayItem` (`self.Layer1`)))
      (else
        (bind _output_get_2 (set `local.TempRoomPool` (`self.RoomNames`)))
        (`KismetArrayLibrary.Array_RemoveItem` _output_get_2 (`|GetArrayItem` (`self.Layer1`) 1))))
    (`KismetArrayLibrary.Array_AddUnique` (`self.Layer2`) (`KismetArrayLibrary.Array_Random` (`local.TempRoomPool`))))
  ;[1 1 1] Debug
  (`KismetSystemLibrary.PrintString` "Layers Built")
  (for _array_element (`self.Layer1`)
    (`KismetSystemLibrary.PrintString` (`KismetStringLibrary.Conv_NameToString` _array_element)))
  (for _array_element_2 (`self.Layer2`)
    (`KismetSystemLibrary.PrintString` (`KismetStringLibrary.Conv_NameToString` _array_element_2))))

(fn `Get Next Rooms`
  (returns (Room1 :type Name) (Room2 :type Name))
  (locals (Destination1 :type Name) (Destination2 :type Name))
  (bind _layer1 (`self.Layer1`))
  (bind _layer2 (`self.Layer2`))
  (switch `int` (`self.PlayerCurrentLayer`)
    (:`0`
      (set `local.Destination1` (`|GetArrayItem` _layer1))
      (set `local.Destination2` (`|GetArrayItem` _layer1 1)))
    (:`1`
      (bind _returnvalue (`GameplayStatics.GetCurrentLevelName` true))
      (switch `int` (`KismetArrayLibrary.Array_Find` _layer1 (`KismetStringLibrary.Conv_StringToName` _returnvalue))
        (:`0`
          (set `local.Destination1` (`|GetArrayItem` _layer2))
          (set `local.Destination2` (`|GetArrayItem` _layer2 1)))
        (:`1`
          (set `local.Destination1` (`|GetArrayItem` _layer2 2))
          (set `local.Destination2` (`|GetArrayItem` _layer2 3)))))
    (:`2`
      (bind _output_get (set `local.Destination1` "TestTile6"))
      (set `local.Destination2` _output_get))
    (:`3`
      (bind _output_get_2 (set `local.Destination1` "TestTile1"))
      (set `local.Destination2` _output_get_2)))
  (return (`local.Destination1`) (`local.Destination2`)))

(fn `IncrimentLayer`
  (bind _playercurrentlayer (`self.PlayerCurrentLayer`))
  (if (< _playercurrentlayer 3)
    (set `self.PlayerCurrentLayer` (+ _playercurrentlayer 1))
    (else
      (set `self.PlayerCurrentLayer` 0))))