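; Player character Blueprint for RuneHunter, with camera-yaw-relative movement, cursor-aimed shooting and an eight-direction dash.
; Tick snaps the mesh to one of four 90-degree facings toward the cursor and picks a walk or idle flipbook from movement flags.
; Input actions set those flags, which also choose the world-axis launch vector for the dash.
; Shooting spawns a default projectile offset toward the cursor, rate-limited by a delay.
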(event `self.ReceiveTick`
  (params (DeltaSeconds :type "Float (single-precision)"))
  (bind _character_flipbook (`self.Character Flipbook`))
  (bind _character_flipbook_2 (`self.Character Flipbook`))
  (bind _yaw (.yaw (`KismetMathLibrary.FindLookAtRotation` (`self.K2_GetActorLocation`) (`.Location` (`GameplayStatics.BreakHitResult` (`PlayerController.GetHitResultUnderCursorByChannel` (`GameplayStatics.GetPlayerController` 0) "TraceTypeQuery3" true))))))
  ;[1 1 1] Rotate Mesh to look at cursor
  (if (`KismetMathLibrary.InRange_FloatFloat` _yaw -135.0 -45.0)
    (set `self.Angle_Facing` 180.0)
    (elif (`KismetMathLibrary.InRange_FloatFloat` _yaw -45.0 45.0)
      (set `self.Angle_Facing` -90.0)
      (elif (`KismetMathLibrary.InRange_FloatFloat` _yaw 45.0 135.0)
        (set `self.Angle_Facing` 0.0)
        (else
          (set `self.Angle_Facing` 90.0)))))
  (`SceneComponent.K2_SetWorldRotation` (`self.Mesh`) (`KismetMathLibrary.MakeRotator` (.roll (`self.K2_GetActorRotation`)) (.pitch (`self.K2_GetActorRotation`)) (`self.Angle_Facing`)) false false)
  ;[1 1 1] Character Animations
  (if (and (`self.MovingUp`) (`self.MovingLeft`))
    (`PaperFlipbookComponent.SetFlipbook` _character_flipbook "/Game/Sprites/Flipbook_Walk_Left_Back.Flipbook_Walk_Left_Back")
    (elif (`self.MovingUp`)
      (`PaperFlipbookComponent.SetFlipbook` _character_flipbook "/Game/Sprites/Flipbook_Walk_Right_Back.Flipbook_Walk_Right_Back")
      (elif (`self.MovingLeft`)
        (`PaperFlipbookComponent.SetFlipbook` (`self.Character Flipbook`) "/Game/Sprites/Flipbook_Walk_Left_Front.Flipbook_Walk_Left_Front")
        (elif (or (`self.MovingDown`) (`self.MovingRight`))
          (`PaperFlipbookComponent.SetFlipbook` _character_flipbook_2 "/Game/Sprites/Flipbook_Walk_Right_Front.Flipbook_Walk_Right_Front")
          (else
            (`PaperFlipbookComponent.SetFlipbook` _character_flipbook_2 "/Game/Sprites/Flipbook_Idle.Flipbook_Idle")))))))

(event `self.ReceiveBeginPlay`
  ;[1 1 1] Debug
  (set `PlayerController.bShowMouseCursor` true (`GameplayStatics.GetPlayerController` 0))
  (set `self.CanShoot` true) ; For shooting action
)

(event `InputAction|MoveUp`
  (params (Key :type "Key Structure"))
  ;[1 1 1] Determine Dash Direction
  (:`Pressed`
    (set `self.MovingUp` true)
    (set `self.MovingDown` false))
  (:`Released`
    (set `self.MovingUp` false)))

(event `InputAction|Shoot`
  (params (Key :type "Key Structure"))
  (bind _returnvalue (`self.K2_GetActorLocation`))
  (bind _returnvalue_2 (`KismetMathLibrary.MakeRotFromZ` (* (`.Y` (`KismetMathLibrary.BreakRotIntoAxes` (`KismetMathLibrary.FindLookAtRotation` _returnvalue (`.Location` (`GameplayStatics.BreakHitResult` (`PlayerController.GetHitResultUnderCursorByChannel` (`GameplayStatics.GetPlayerController` 0) "TraceTypeQuery3" true)))))) -1.0)))
  ;[1 1 1] Basic Shooting
  (:`Pressed`
    (if (`self.CanShoot`)
      (`|SpawnActorFromClass` "/Game/Projectile_DefaultBP.Projectile_DefaultBP_C" (`KismetMathLibrary.MakeTransform` (+ _returnvalue (`KismetMathLibrary.GreaterGreater_VectorRotator` (`KismetMathLibrary.MakeVector` 200.0) _returnvalue_2)) _returnvalue_2) "Undefined" "OverrideRootScale" null null)
      ;;[1 1 1] Delay for shoot action
      (set `self.CanShoot` false)
      (`KismetSystemLibrary.Delay` (`self.Delay_Time`))
      (set `self.CanShoot` true))))

(event `InputAxis|MoveForward` :overrideparent false
  (params (AxisValue :type "Float (single-precision)"))
  ;[1 1 1] Basic Movement Rotated to Camera
  (`self.AddMovementInput` (`KismetMathLibrary.GetForwardVector` (`KismetMathLibrary.MakeRotator` 0.0 0.0 (.yaw (`self.GetControlRotation`)))) AxisValue))

(event `InputAction|MoveDown`
  (params (Key :type "Key Structure"))
  ;[1 1 1] Determine Dash Direction
  (:`Pressed`
    (set `self.MovingDown` true)
    (set `self.MovingUp` false))
  (:`Released`
    (set `self.MovingDown` false)))

(event `InputAction|MoveRight`
  (params (Key :type "Key Structure"))
  ;[1 1 1] Determine Dash Direction
  (:`Pressed`
    (set `self.MovingRight` true)
    (set `self.MovingLeft` false))
  (:`Released`
    (set `self.MovingRight` false)))

(event `InputAction|MoveLeft`
  (params (Key :type "Key Structure"))
  ;[1 1 1] Determine Dash Direction
  (:`Pressed`
    (set `self.MovingLeft` true)
    (set `self.MovingRight` false))
  (:`Released`
    (set `self.MovingLeft` false)))

(event `InputAxis|MoveRight` :overrideparent false
  (params (AxisValue :type "Float (single-precision)"))
  ;[1 1 1] Basic Movement Rotated to Camera
  (`self.AddMovementInput` (`KismetMathLibrary.GetRightVector` (`KismetMathLibrary.MakeRotator` 0.0 0.0 (.yaw (`self.GetControlRotation`)))) AxisValue))

(event `InputAction|Dash`
  (params (Key :type "Key Structure"))
  (bind _dash_speed (`self.Dash_Speed`))
  (bind _dash_speed_2 (`self.Dash_Speed`))
  (bind _returnvalue (`KismetMathLibrary.MakeVector` 0.0 _dash_speed))
  (bind _returnvalue_2 (`KismetMathLibrary.MakeVector` _dash_speed_2))
  (bind _returnvalue_3 (`KismetMathLibrary.MakeVector` (* _dash_speed_2 -1.0)))
  (bind _returnvalue_4 (`KismetMathLibrary.MakeVector` 0.0 (* _dash_speed -1.0)))
  ;[1 1 1] 8 Directional Dash
  (:`Pressed`
    (if (`self.MovingUp`)
      (if (`self.MovingRight`)
        (set `self.Dash_Vector` (+ _returnvalue_2 _returnvalue))
        (elif (`self.MovingLeft`)
          (set `self.Dash_Vector` (+ _returnvalue_2 _returnvalue_4))
          (else
            (set `self.Dash_Vector` _returnvalue_2))))
      (`self.LaunchCharacter` (`self.Dash_Vector`) :!label _label)
      (elif (`self.MovingDown`)
        (if (`self.MovingRight`)
          (set `self.Dash_Vector` (+ _returnvalue_3 _returnvalue))
          (goto _label)
          (elif (`self.MovingLeft`)
            (set `self.Dash_Vector` (+ _returnvalue_3 _returnvalue_4))
            (goto _label)
            (else
              (set `self.Dash_Vector` _returnvalue_3)
              (goto _label))))
        (elif (`self.MovingRight`)
          (set `self.Dash_Vector` _returnvalue)
          (goto _label)
          (elif (`self.MovingLeft`)
            (set `self.Dash_Vector` _returnvalue_4)
            (goto _label)))))))

(fn `UserConstructionScript`)